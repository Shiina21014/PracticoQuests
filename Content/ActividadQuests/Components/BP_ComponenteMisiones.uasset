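; Quest component that tracks running missions and their objective progress.
; AgregarMision copies a definition's objectives into a runtime struct in MisionesActivas, rejecting invalid definitions and duplicate IDs.
; Objective events from the BP_EstadoMisiones GameState add to only the first type-and-target match in unfinished missions.
; Once all objectives meet their required counts, the mission is marked completed but stays listed; dispatchers announce start, progress and completion.
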(event `self.ReceiveBeginPlay`
  (bind _asbp_estado_misiones (cast `/Game/ActividadQuests/Components/BP_EstadoMisiones` (`GameplayStatics.GetGameState`)))
  (add `/Game/ActividadQuests/Components/BP_EstadoMisiones.AlReportarEventoObjetivo` _asbp_estado_misiones (delegate `RecibirEventoObjetivo`)))

(event `RecibirEventoObjetivo`
  (params (TipoObjetivo :type "/Game/ActividadQuests/Types/E_TipoObjetivoMision Enum" :default "NewEnumerator0") (IDDestino :type Name) (Cantidad :type Integer))
  (`self.ActualizarProgresoObjetivo` TipoObjetivo IDDestino Cantidad))

(fn `ActualizarProgresoObjetivo`
  (params (TipoObjetivo :type "/Game/ActividadQuests/Types/E_TipoObjetivoMision Enum" :default "NewEnumerator0") (IDDestino :type Name) (Cantidad :type Integer))
  (locals (MisionLocal :type "/Game/ActividadQuests/Types/ST_MisionEnEjecucion Structure") (ObjetivosLocales :type "Array of /Game/ActividadQuests/Types/ST_ObjetivoMision Structure") (ObjetivoLocal :type "/Game/ActividadQuests/Types/ST_ObjetivoMision Structure"))
  (bind _misionesactivas (`self.MisionesActivas`))
  (bind _misionlocal (`local.MisionLocal`))
  (bind _objetivoslocales (`local.ObjetivosLocales`))
  (bind _objetivolocal (`local.ObjetivoLocal`))
  (bind (_idmision _definicionmision _objetivos _estaactiva _estacompletada) (break `/Game/ActividadQuests/Types/ST_MisionEnEjecucion` _misionlocal))
  (bind (_idobjetivo _nombre _tipoobjetivo _iddestino _cantidadrequerida _cantidadactual) (break `/Game/ActividadQuests/Types/ST_ObjetivoMision` _objetivolocal))
  (for (_array_element _array_index) _misionesactivas
    (set `local.MisionLocal` _array_element)
    (if (and _estaactiva (not _estacompletada))
      (set `local.ObjetivosLocales` _objetivos)
      (for (_array_element_2 _array_index_2) _objetivoslocales
        (set `local.ObjetivoLocal` _array_element_2)
        (if (and (`|EnumEquality` _tipoobjetivo TipoObjetivo) (== _iddestino IDDestino))
          (bind _structout (setmembers `/Game/ActividadQuests/Types/ST_ObjetivoMision` :`StructRef` _objetivolocal :`CantidadActual` (+ _cantidadactual Cantidad)))
          (set `local.ObjetivoLocal` _structout)
          (`KismetArrayLibrary.Array_Set` _objetivoslocales _array_index_2 _objetivolocal)
          (bind _structout_2 (setmembers `/Game/ActividadQuests/Types/ST_MisionEnEjecucion` :`StructRef` _misionlocal :`Objetivos` _objetivoslocales))
          (set `local.MisionLocal` _structout_2)
          (`KismetArrayLibrary.Array_Set` _misionesactivas _array_index _misionlocal)
          (`self.AlCambiarProgreso` _misionlocal)
          (`self.ComprobarMisionCompletada` _array_index)
          (return))))))

(fn `AgregarMision`
  (params (DefinicionMision :type "/Game/ActividadQuests/Definitions/PDA_DefinicionMision Object Reference"))
  (returns (Agregada :type Boolean))
  (bind _idmision (`/Game/ActividadQuests/Definitions/PDA_DefinicionMision.IDMision` DefinicionMision))
  (bind _st_misionenejecucion (make `/Game/ActividadQuests/Types/ST_MisionEnEjecucion` _idmision DefinicionMision (`/Game/ActividadQuests/Definitions/PDA_DefinicionMision.Objetivos` DefinicionMision) true))
  (if (`KismetSystemLibrary.IsValid` DefinicionMision)
    (bind _encontrada (`self.BuscarMisionPorID` _idmision))
    (if _encontrada
      (return false)
      (else
        (`KismetArrayLibrary.Array_Add` (`self.MisionesActivas`) _st_misionenejecucion)
        (`self.AlIniciarMision` _st_misionenejecucion)
        (return true)))
    (else
      (return false))))

(fn `BuscarMisionPorID`
  (params (IDMisionBuscado :type Name))
  (returns (Encontrada :type Boolean) (DatosMision :type "/Game/ActividadQuests/Types/ST_MisionEnEjecucion Structure") (IndiceMision :type Integer))
  (for (_array_element _array_index) (`self.MisionesActivas`)
    (if (== (`.IDMision_7_B3389A8E4AF0A37AF43828B2B3C12D40` (break `/Game/ActividadQuests/Types/ST_MisionEnEjecucion` _array_element)) IDMisionBuscado)
      (return true _array_element _array_index)))
  (return false (struct) -1))

(fn `ComprobarMisionCompletada`
  (params (IndiceMision :type Integer))
  (locals (MisionComprobada :type "/Game/ActividadQuests/Types/ST_MisionEnEjecucion Structure"))
  (bind _misionesactivas (`self.MisionesActivas`))
  (bind _misioncomprobada (`local.MisionComprobada`))
  (set `local.MisionComprobada` (`|GetArrayItem` _misionesactivas IndiceMision))
  (for _array_element (`.Objetivos_11_495CAC2E402162B3BC29B28FDE7CC65E` (break `/Game/ActividadQuests/Types/ST_MisionEnEjecucion` _misioncomprobada))
    (bind (_idobjetivo _nombre _tipoobjetivo _iddestino _cantidadrequerida _cantidadactual) (break `/Game/ActividadQuests/Types/ST_ObjetivoMision` _array_element))
    (if (not (>= _cantidadactual _cantidadrequerida))
      (return)))
  (bind _structout (setmembers `/Game/ActividadQuests/Types/ST_MisionEnEjecucion` :`StructRef` _misioncomprobada :`EstaActiva` false :`EstaCompletada` true))
  (set `local.MisionComprobada` _structout)
  (`KismetArrayLibrary.Array_Set` _misionesactivas IndiceMision _misioncomprobada)
  (`self.AlCompletarMision` _misioncomprobada)
  (return))